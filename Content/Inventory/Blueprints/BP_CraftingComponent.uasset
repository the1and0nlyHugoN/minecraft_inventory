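; BP_CraftingComponent is a component that sets up the slot objects for a crafting inventory on the first-person character controller.
; On BeginPlay it casts its owner to FirstPersonCharacterController and caches it.
; The CreateInventory event fills the Inventory array with SlotClass objects, one per cell of the Size grid, and creates a separate crafting result slot.
; All slots are constructed with the controller as Outer, and no recipe logic is present.
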(event EventCreateInventory
  (params (SlotClass :type Slot%20Class%20Reference))
  (bind _size (Variables|Default|GetSize))
  (bind (_x _y) (Math|Vector2D|BreakVector2D _size))
  (for _index (range 0 (- (Math|Float|Truncate _x) 1))
    (for _index_2 (range 0 (- (Math|Float|Truncate _y) 1))
      (bind _returnvalue (Game|ConstructObjectfromClass (Variables|Default|GetSlotClass) (Variables|Default|GetOwnerController)))
      (Utilities|Array|Add (Variables|Default|GetInventory) _returnvalue)))
  (bind _returnvalue_2 (Game|ConstructObjectfromClass "/Game/Inventory/Blueprints/BP_CraftingResultSlot.BP_CraftingResultSlot_C" (Variables|Default|GetOwnerController)))
  (Variables|Default|SetCraftedSlot _returnvalue_2))

(event EventBeginPlay
  (bind _asfirst_person_character_controller (Utilities|Casting|CastToFirstPersonCharacterController (Components|GetOwner)))
  (Variables|Default|SetOwnerController _asfirst_person_character_controller))