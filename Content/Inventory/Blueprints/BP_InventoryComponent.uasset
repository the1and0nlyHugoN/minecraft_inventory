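; Inventory component owned by the first-person controller, holding a collection of slot objects and filling it with items.
; BeginPlay caches the owner as a FirstPersonCharacterController, which becomes the outer for constructed slots.
; CreateInventory builds one SlotClass object per cell of the Size X by Y grid into a flat Inventory array.
; LoadInventory passes every row of the DT_Item data table to TryAddToInventory, ignoring the result.
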(event EventCreateInventory
  (params (SlotClass :type Slot%20Class%20Reference))
  (bind _size (Variables|Default|GetSize))
  (bind (_x _y) (Math|Vector2D|BreakVector2D _size))
  (for _index (range 0 (- (Math|Float|Truncate _x) 1))
    (for _index_2 (range 0 (- (Math|Float|Truncate _y) 1))
      (bind _returnvalue (Game|ConstructObjectfromClass (Variables|Default|GetSlotClass) (Variables|Default|GetOwnerController)))
      (Utilities|Array|Add (Variables|Default|GetInventory) _returnvalue))))

(event EventBeginPlay
  (bind _asfirst_person_character_controller (Utilities|Casting|CastToFirstPersonCharacterController (Components|GetOwner)))
  (Variables|Default|SetOwnerController _asfirst_person_character_controller))

(event EventLoadInventory
  (bind _outrownames (DataTable|GetDataTableRowNames "/Game/Inventory/Data/DT_Item.DT_Item"))
  (for _array_element _outrownames
    (bind _returnvalue (Utilities|GetDataTableRow "/Game/Inventory/Data/DT_Item.DT_Item" _array_element)
      (:then
        (bind _returnvalue_2 (Class|InventoryComponent|TryAddtoInventory _returnvalue))
        (if _returnvalue_2
          _)))))